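; RTS HUD that provides drag-box (marquee) selection of BP_RTS_Unit actors.
; Input start, hold and end events clear the previous selection, track the mouse corners and pass the final list to BP_RTS_PlayerController.
; While dragging, DrawHUD draws the translucent rectangle and uses GetActorsInSelectionRectangle to add units inside it and deselect those that leave, updating their selected state live.
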(event `self.ReceiveBeginPlay`
  (set `self.PlayerController` (cast `/Game/Player/BP_RTS_PlayerController` (`GameplayStatics.GetPlayerController` 0) :!pure true)))

(event `/Game/Core/BPI_MarqueeSelector.OnInputStart`
  (bind (_locationx _locationy) (`PlayerController.GetMousePosition` (`self.PlayerController`)))
  (`self.SetActorTickEnabled` true)
  (if (>= (`KismetArrayLibrary.Array_Length` (`self.SelectedUnits`)) 0)
    (for _array_element (`self.SelectedUnits`)
      (`/Game/Characters/BP_RTS_Unit.Set Selected Unit` _array_element false)
      (set `/Game/Characters/BP_RTS_Unit.IsSelected` false _array_element))
    (`KismetArrayLibrary.Array_Clear` (`self.SelectedUnits`)))
  (bind _output_get (set `self.ClickLocation` (`KismetMathLibrary.MakeVector2D` _locationx _locationy)))
  (set `self.HoldingLocation` _output_get)
  (set `self.IsDrawing` true))

(event `/Game/Core/BPI_MarqueeSelector.OnInputHold`
  (bind (_locationx _locationy) (`PlayerController.GetMousePosition` (`self.PlayerController`)))
  (set `self.HoldingLocation` (`KismetMathLibrary.MakeVector2D` _locationx _locationy)))

(event `/Game/Core/BPI_MarqueeSelector.OnInputEnd`
  (params (HoldTime :type "Float (single-precision)"))
  (`self.SetActorTickEnabled` false)
  (set `self.IsDrawing` false)
  (`/Game/Player/BP_RTS_PlayerController.SelectUnits` (`self.PlayerController`) (`self.SelectedUnits`)))

(event `self.ReceiveDrawHUD`
  (params (SizeX :type Integer) (SizeY :type Integer))
  (if (`self.IsDrawing`)
    (`|ExecutionSequence`
      (:`then_0`
        (`self.DrawMarquee`))
      (:`then_1`
        (`self.SelectUnits`))
      (:`then_2`
        (`self.UnselectUnits`)))))

(event `DrawMarquee`
  (bind (_x _y) (`KismetMathLibrary.BreakVector2D` (`self.ClickLocation`)))
  (bind (_x_2 _y_2) (`KismetMathLibrary.BreakVector2D` (`self.ClickLocation`)))
  (bind (_x_3 _y_3) (`KismetMathLibrary.BreakVector2D` (`self.HoldingLocation`)))
  (bind (_x_4 _y_4) (`KismetMathLibrary.BreakVector2D` (- (`self.HoldingLocation`) (`self.ClickLocation`))))
  (`self.DrawRect` (struct :`A` 1) _x_2 _y_2)
  (`self.DrawRect` (struct :`A` 1) _x_3 _y_3)
  (`self.DrawRect` (struct :`R` 0.459215 :`G` 1.0 :`B` 0.388603 :`A` 0.6) _x _y _x_4 _y_4))

(event `SelectUnits`
  (for _array_element (`self.GetActorsInSelectionRectangle` "/Game/Characters/BP_RTS_Unit.BP_RTS_Unit_C" (`self.ClickLocation`) (`self.HoldingLocation`) false)
    (bind _asbp_rts_unit (cast `/Game/Characters/BP_RTS_Unit` _array_element))
    (`KismetArrayLibrary.Array_AddUnique` (`self.SelectedUnits`) _asbp_rts_unit)
    (`/Game/Characters/BP_RTS_Unit.Set Selected Unit` _asbp_rts_unit true)))

(event `UnselectUnits`
  (for _array_element (`self.SelectedUnits`)
    (if (not (`KismetArrayLibrary.Array_Contains` (`self.GetActorsInSelectionRectangle` "/Game/Characters/BP_RTS_Unit.BP_RTS_Unit_C" (`self.ClickLocation`) (`self.HoldingLocation`) false) _array_element))
      (`/Game/Characters/BP_RTS_Unit.Set Selected Unit` _array_element false)
      (`KismetArrayLibrary.Array_RemoveItem` (`self.SelectedUnits`) _array_element))))

(fn `UserConstructionScript`)