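; Map actor for the RTS command interface that displays a map surface and hosts miniature markers for units.
; Construction applies a dynamic instance of M_Map to the mesh.
; A player capsule entering or leaving the box switches the RTS controller's CommandMode and sets or clears its focused map.
; AddUnitToMap spawns a BP_MapUnits linked to its unit, offset from the map by the unit's world XY scaled down fifteenfold.
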(event `self.Box.OnComponentBeginOverlap`
  (params (OverlappedComponent :type "PrimitiveComponent Object Reference") (OtherActor :type "Actor Object Reference") (OtherComp :type "PrimitiveComponent Object Reference") (OtherBodyIndex :type Integer) (bFromSweep :type Boolean) (SweepResult :type "HitResult Structure (by ref)"))
  (bind _returnvalue (`self.GetInstigatorController` OtherActor))
  (bind _asbp_rts_player_controller (cast `/Game/Player/BP_RTS_PlayerController` _returnvalue :!pure true))
  (if (and (`Controller.IsPlayerController` _returnvalue) (== (`GameplayStatics.GetObjectClass` OtherComp) "/Script/Engine.CapsuleComponent"))
    (set `/Game/Player/BP_RTS_PlayerController.CommandMode` "NewEnumerator2" _asbp_rts_player_controller)
    (set `/Game/Player/BP_RTS_PlayerController.CurrentMapFocused` self _asbp_rts_player_controller)))

(event `self.Box.OnComponentEndOverlap`
  (params (OverlappedComponent :type "PrimitiveComponent Object Reference") (OtherActor :type "Actor Object Reference") (OtherComp :type "PrimitiveComponent Object Reference") (OtherBodyIndex :type Integer))
  (bind _returnvalue (`self.GetInstigatorController` OtherActor))
  (bind _asbp_rts_player_controller (cast `/Game/Player/BP_RTS_PlayerController` _returnvalue :!pure true))
  (if (and (`Controller.IsPlayerController` _returnvalue) (== (`GameplayStatics.GetObjectClass` OtherComp) "/Script/Engine.CapsuleComponent"))
    (set `/Game/Player/BP_RTS_PlayerController.CommandMode` "NewEnumerator1" _asbp_rts_player_controller)
    (set `/Game/Player/BP_RTS_PlayerController.CurrentMapFocused` null _asbp_rts_player_controller)))

(fn `AddUnitToMap`
  (params (Instigator :type "Pawn Object Reference"))
  (bind (_returnvalue_x _returnvalue_y _returnvalue_z) (`KismetMathLibrary.BreakVector` (`self.K2_GetActorLocation`)))
  (bind (_returnvalue_x_2 _returnvalue_y_2) (`KismetMathLibrary.BreakVector` (`self.K2_GetActorLocation` Instigator)))
  (bind _returnvalue (`|SpawnActorFromClass` "/Game/HUD/BP_MapUnits.BP_MapUnits_C" (`KismetMathLibrary.MakeTransform` (`KismetMathLibrary.MakeVector` (+ (/ _returnvalue_x_2 15.0) _returnvalue_x) (+ (/ _returnvalue_y_2 15.0) _returnvalue_y) _returnvalue_z)) "Undefined" "OverrideRootScale" self Instigator))
  (set `/Game/HUD/BP_MapUnits.UnitOwner` Instigator _returnvalue))

(fn `UserConstructionScript`
  (bind _returnvalue (`KismetMaterialLibrary.CreateDynamicMaterialInstance` "/Game/HUD/M_Map.M_Map"))
  (bind _output_get (set `self.MapMaterial` _returnvalue))
  (`PrimitiveComponent.SetMaterial` (`self.StaticMesh`) 0 _output_get))