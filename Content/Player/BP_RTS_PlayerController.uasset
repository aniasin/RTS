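; RTS player controller that turns left-click input into selection messages for the marquee selector HUD.
; On press it notifies the HUD, on each tick while held it sends hold messages and accumulates hold time, and on release it passes that time to the HUD.
; A SelectUnits function stores the given units as the current selection.
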(event `self.ReceiveTick`
  (params (DeltaSeconds :type "Float (single-precision)"))
  (if (`self.IsHoldingInput`)
    (set `self.HoldingTime` (+ (`self.HoldingTime`) DeltaSeconds))
    (message `/Game/Core/BPI_MarqueeSelector.OnInputHold` (`self.HUDRef`))))

(event `self.ReceiveBeginPlay`
  (set `self.HUDRef` (cast `/Game/HUD/BP_HUD_MarqueeSelector` (`self.GetHUD`) :!pure true)))

(event `InputAction|LeftClick`
  (params (Key :type "Key Structure"))
  (:`Pressed`
    (message `/Game/Core/BPI_MarqueeSelector.OnInputStart` (`self.HUDRef`))
    (set `self.HoldingTime` 0.0)
    (set `self.IsHoldingInput` true))
  (:`Released`
    (message `/Game/Core/BPI_MarqueeSelector.OnInputEnd` (`self.HUDRef`) (`self.HoldingTime`))
    (set `self.IsHoldingInput` false)))

(fn `SelectUnits`
  (params (Units :type "Array of /Game/Characters/BP_RTS_Unit Object Reference"))
  (set `self.SelectedUnits` Units))

(fn `UserConstructionScript`)